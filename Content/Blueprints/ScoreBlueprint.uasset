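; ScoreBlueprint is an input-enabled actor that keeps a Score counter and prints it as debug text.
; BeginPlay enables input from player controller 0, and each press of R calls EditScore.
; EditScore adds a fixed 5 to Score and prints the result, ignoring its NewParam argument.
; The construction script also calls EditScore, so construction itself increments and prints the score.
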(event EventBeginPlay
  (Input|EnableInput (Game|GetPlayerController 0)))

(event Collision|EventActorBeginOverlap
  (params (OtherActor :type Actor%20Object%20Reference)))

(event EventTick
  (params (DeltaSeconds :type Float%20%28single-precision%29)))

(event Input|KeyboardEvents|R
  (params (Key :type Key%20Structure :default "None"))
  (:Pressed
    (CallFunction|EditScore)))

(fn ConstructionScript
  (CallFunction|EditScore))

(fn EditScore
  (params (NewParam :type Integer))
  (bind _output_get (Variables|Default|SetScore (+ (Variables|Default|GetScore) 5)))
  (Development|PrintString (Utilities|String|ToString(Integer) _output_get)))