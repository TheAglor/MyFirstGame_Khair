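; Enemy character Blueprint that carries a health bar widget, refreshed every Tick from CurrentHP over MaxHP.
; It also holds player-style input for movement along control rotation, camera look, and aiming that sets IsAiming and plays or reverses a Zoom timeline.
; The Zoom timeline's output drives nothing, and a muzzle line trace for hit confirmation is left disconnected, so the file implements no shooting or damage.
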(event EventTick
  (params (DeltaSeconds :type Float%20%28single-precision%29))
  (bind _aswb_health_bar (Utilities|Casting|CastToWB_HealthBar (UserInterface|GetWidget (Variables|Default|GetHP_Bar))))
  (Progress|SetPercent (Variables|/Game/Blueprints/WB_HealthBar.WB_HealthBar_C|GetHealthBar _aswb_health_bar) (/ (Variables|Default|GetCurrentHP) (Variables|Default|GetMaxHP))))

(event Input|ActionEvents|InputActionAimWeapon
  (params (Key :type Key%20Structure :default "None"))
  ;[1 1 1] Weapon Aim Input
  (:Pressed
    (Variables|Default|SetisAiming true)
    (bind _lerp (Timeline|Zoom PlayFromStart)))
  (:Released
    (Variables|Default|SetisAiming false)
    (Timeline|Zoom Reverse)))

(event Input|AxisEvents|InputAxisGoForwardBackward
  (params (AxisValue :type Float%20%28single-precision%29))
  ;[0 0 0] Movement
  (Pawn|Input|AddMovementInput (Math|Vector|GetForwardVector (Math|Rotator|MakeRotator 0.0 0.0 (.yaw (Pawn|GetControlRotation :!class /Script/Engine.Pawn)))) AxisValue false))

(event Input|AxisEvents|InputAxisGoRightLeft
  (params (AxisValue :type Float%20%28single-precision%29))
  (bind _returnvalue (Pawn|GetControlRotation :!class /Script/Engine.Pawn))
  ;[0 0 0] Movement
  (Pawn|Input|AddMovementInput (Math|Vector|GetRightVector (Math|Rotator|MakeRotator (.roll _returnvalue) 0.0 (.yaw _returnvalue))) AxisValue false))

(event Input|AxisEvents|InputAxisCameraUpDown
  (params (AxisValue :type Float%20%28single-precision%29))
  ;[1 1 1] Camera
  (Pawn|Input|AddControllerPitchInput AxisValue))

(event Input|AxisEvents|InputAxisCameraRightLeft
  (params (AxisValue :type Float%20%28single-precision%29))
  ;[1 1 1] Camera
  (Pawn|Input|AddControllerYawInput AxisValue))

(fn ConstructionScript)